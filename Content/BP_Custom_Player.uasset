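; BP_Custom_Player is the player controller that handles Enhanced Input for first-player movement, looking, jumping and door interaction.
; It adds IMC_Player on BeginPlay and drives the player character, moving it relative to BP_Player's camera yaw.
; Interact runs a short, debug-drawn Visibility line trace from that camera.
; A hit BP_Door opens, while a hit BP_Door_crying_baby_2_Blueprint receives its close-door event.
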(event `EnhancedInput|/Game/input/actions/IA_Jump`
  (params (ActionValue :type Boolean) (ElapsedSeconds :type "Float (double-precision)") (TriggeredSeconds :type "Float (double-precision)") (InputAction :type "InputAction Object Reference" :default "/Game/input/actions/IA_Jump.IA_Jump"))
  (:`Triggered`
    (`Character.Jump` (`GameplayStatics.GetPlayerCharacter` 0))))

(event `self.ReceiveBeginPlay`
  (`EnhancedInputSubsystemInterface.AddMappingContext` (subsystem `EnhancedInputLocalPlayerSubsystem`) "/Game/input/IMC_Player.IMC_Player" 0 (struct)))

(event `EnhancedInput|/Game/input/actions/IA_Move`
  (params (ActionValue :type "Vector2D Structure") (ElapsedSeconds :type "Float (double-precision)") (TriggeredSeconds :type "Float (double-precision)") (InputAction :type "InputAction Object Reference" :default "/Game/input/actions/IA_Move.IA_Move"))
  (bind _returnvalue (`GameplayStatics.GetPlayerCharacter` 0))
  (:`Triggered`
    (bind _asbp_player (cast `/Game/BP_Player` _returnvalue))
    (bind (_returnvalue_roll _returnvalue_pitch _returnvalue_yaw) (`KismetMathLibrary.BreakRotator` (`SceneComponent.K2_GetComponentRotation` (`/Game/BP_Player.Character_Camera` _asbp_player))))
    (`Pawn.AddMovementInput` _returnvalue (`KismetMathLibrary.GetForwardVector` (`KismetMathLibrary.MakeRotator` 0.0 0.0 _returnvalue_yaw)) ActionValue_X false)
    (`Pawn.AddMovementInput` _returnvalue (`KismetMathLibrary.GetRightVector` (`KismetMathLibrary.MakeRotator` 0.0 0.0 _returnvalue_yaw)) ActionValue_Y false)))

(event `EnhancedInput|/Game/input/actions/IA_Look`
  (params (ActionValue :type "Vector2D Structure") (ElapsedSeconds :type "Float (double-precision)") (TriggeredSeconds :type "Float (double-precision)") (InputAction :type "InputAction Object Reference" :default "/Game/input/actions/IA_Look.IA_Look"))
  (:`Triggered`
    (`self.AddYawInput` ActionValue_X)
    (`Pawn.AddControllerPitchInput` (`GameplayStatics.GetPlayerCharacter` 0) ActionValue_Y)))

(event `EnhancedInput|/Game/input/actions/IA_Interact`
  (params (ActionValue :type Boolean) (ElapsedSeconds :type "Float (double-precision)") (TriggeredSeconds :type "Float (double-precision)") (InputAction :type "InputAction Object Reference" :default "/Game/input/actions/IA_Interact.IA_Interact"))
  (:`Started`
    (bind _asbp_player (cast `/Game/BP_Player` (`GameplayStatics.GetPlayerCharacter` 0)))
    (bind _character_camera (`/Game/BP_Player.Character_Camera` _asbp_player))
    (bind _returnvalue (`SceneComponent.K2_GetComponentLocation` _character_camera))
    (bind _outhit (`KismetSystemLibrary.LineTraceSingle` :`Start` _returnvalue :`End` (+ _returnvalue (* (`SceneComponent.GetForwardVector` _character_camera) 200.0)) :`TraceChannel` "TraceTypeQuery1" :`DrawDebugType` "ForDuration"))
    (bind _asbp_door (cast `/Game/BP_Door` (`.HitActor` (`GameplayStatics.BreakHitResult` _outhit)))
      (:`then`
        (`/Game/BP_Door.openDoor` _asbp_door))
      (:`CastFailed`
        (bind _asbp_door_crying_baby_2_blueprint (cast `/Game/exercice_layers_of_fear/BP_Door_crying_baby_2_Blueprint` (`.HitActor` (`GameplayStatics.BreakHitResult` _outhit))))
        (`/Game/exercice_layers_of_fear/BP_Door_crying_baby_2_Blueprint.Close_Door_Event` _asbp_door_crying_baby_2_blueprint)))))

(fn `UserConstructionScript`)