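; BP_Door is a two-leaf door that swings open and closed.
; The openDoor event toggles IsClosed and plays or reverses the OpenDoorAnimation timeline, which drives both meshes' yaw using RotationAngle.
; The construction script poses the leaves and timeline from IsClosed, though its hard-coded yaws differ from those the timeline produces.
; Older snap-toggle and initial-rotation logic remains unconnected.
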(event `openDoor`
  (if (`self.IsClosed`)
    (set `self.IsClosed` false)
    (bind (_direction _newtrack_0) (`Timeline|Open Door Animation` :!label _label)
      (:`Update`
        (`SceneComponent.K2_SetRelativeRotation` (`self.Door_3_StaticMeshComponent0`) (`KismetMathLibrary.MakeRotator` 0.0 0.0 (* _newtrack_0 (`self.rotation angle`) -80.0)) false false)
        (`SceneComponent.K2_SetRelativeRotation` (`self.Door_4_StaticMeshComponent0`) (`KismetMathLibrary.MakeRotator` 0.0 0.0 (`KismetMathLibrary.Lerp` 180.0 (+ (`self.rotation angle`) 180.0) _newtrack_0)) false false)))
    (else
      (set `self.IsClosed` true)
      (goto _label :!via `Reverse`))))

(event `self.ReceiveBeginPlay`)

(fn `UserConstructionScript`
  (`SceneComponent.K2_SetRelativeRotation` (`self.Door_3_StaticMeshComponent0`) (`KismetMathLibrary.MakeRotator` 0.0 0.0 (select `bool` (`self.IsClosed`) :`false` 260.0 :`true` 180.0 :!type "Float (single-precision)")) false false)
  (`SceneComponent.K2_SetRelativeRotation` (`self.Door_4_StaticMeshComponent0`) (`KismetMathLibrary.MakeRotator` 0.0 0.0 (select `bool` (`self.IsClosed`) :`false` -80.0 :!type "Float (single-precision)")) false false)
  (`TimelineComponent.SetNewTime` (`self.Open Door Animation`) (select `bool` (`self.IsClosed`) :`false` 1.0 :!type "Float (single-precision)")))