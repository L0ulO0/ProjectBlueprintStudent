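; Horror double-door Blueprint that plays a demonic baby cry and can slam its two door leaves shut.
; The first overlap of its box trigger plays the positional crying sound once, if IsAllreadyPlay is false.
; Close_Door_Event, not called within this graph, runs a timeline whose update sets both leaves to fixed opposite yaws, without interpolation, and plays a slam sound once.
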(event `Close_Door_Event`
  (if true
    (`Timeline|Close_Door_Event_Animation`
      (:`Update`
        (`SceneComponent.K2_SetRelativeRotation` (`self.Door_crying_baby_2_StaticMeshComponent0`) (`KismetMathLibrary.MakeRotator` 0.0 0.0 -90.0) false false)
        (`SceneComponent.K2_SetRelativeRotation` (`self.Door_Crying_baby_1_StaticMeshComponent0`) (`KismetMathLibrary.MakeRotator` 0.0 0.0 90.0) false false)
        (`/Engine/EditorBlueprintResources/StandardMacros.DoOnce` false
          (:`Completed`
            (`GameplayStatics.PlaySoundAtLocation` "/Game/exercice_layers_of_fear/Door_Slam_Sound_Effect.Door_Slam_Sound_Effect" (0.0 0.0 0.0) (struct) 1.0 1.0 0.0 "/Game/exercice_layers_of_fear/Crying_audio.Crying_audio" null null null)))))))

(event `self.Box.OnComponentBeginOverlap`
  (params (OverlappedComponent :type "PrimitiveComponent Object Reference") (OtherActor :type "Actor Object Reference") (OtherComp :type "PrimitiveComponent Object Reference") (OtherBodyIndex :type Integer) (bFromSweep :type Boolean) (SweepResult :type "HitResult Structure (by ref)"))
  (`/Engine/EditorBlueprintResources/StandardMacros.DoOnce` false
    (:`Completed`
      (if (not (`self.Is_allready_Play`))
        (`GameplayStatics.PlaySoundAtLocation` "/Game/exercice_layers_of_fear/😱_Scary_DEMON_Baby_Crying__Horror_Sounds__FREE___HD__😱.😱_Scary_DEMON_Baby_Crying__Horror_Sounds__FREE___HD__😱" (0.0 0.0 0.0) (struct) 1.0 1.0 0.0 "/Game/exercice_layers_of_fear/Crying_audio.Crying_audio" null null null)))))

(fn `UserConstructionScript`)